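; PowerBP is an interactable painting that shows the player a text widget.
; On BeginPlay it creates an interact prompt and the painting text widget.
; Its Box collider adds the prompt to the viewport when the player character enters and removes it on exit.
; Interact adds or removes the text widget based on the Active flag, then flips and returns that flag.
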(event `self.ReceiveBeginPlay`
  (bind _returnvalue (`|CreateWidget` "/Game/Widgets/PowerPaintingText.PowerPaintingText_C"))
  (bind _returnvalue_2 (`|CreateWidget` "/Game/Widgets/P_Interact.P_Interact_C"))
  (set `self.InteractPrompt` _returnvalue_2)
  (set `self.PowerPaintingText` _returnvalue))

(event `self.Box.OnComponentBeginOverlap`
  (params (OverlappedComponent :type "PrimitiveComponent Object Reference") (OtherActor :type "Actor Object Reference") (OtherComp :type "PrimitiveComponent Object Reference") (OtherBodyIndex :type Integer) (bFromSweep :type Boolean) (SweepResult :type "HitResult Structure (by ref)"))
  ;[1 1 1] When player Enters Box collider for painting
  (if (== OtherActor (`GameplayStatics.GetPlayerCharacter` 0))
    (`UserWidget.AddToViewport` (`self.InteractPrompt`) 0)))

(event `self.Box.OnComponentEndOverlap`
  (params (OverlappedComponent :type "PrimitiveComponent Object Reference") (OtherActor :type "Actor Object Reference") (OtherComp :type "PrimitiveComponent Object Reference") (OtherBodyIndex :type Integer))
  ;[1 1 1] When player Enters Box collider for painting
  (if (== (`GameplayStatics.GetPlayerCharacter` 0) OtherActor)
    (`Widget.RemoveFromParent` (`self.InteractPrompt`))))

(fn `Interact`
  (params (Interactor :type "Character Object Reference"))
  (returns (`Did Interact?` :type Boolean))
  (bind _powerpaintingtext (`self.PowerPaintingText`))
  (bind _active (`self.Active`))
  (if _active
    (`UserWidget.AddToViewport` _powerpaintingtext 0)
    (else
      (`Widget.RemoveFromParent` _powerpaintingtext)))
  (bind _output_get (set `self.Active` (not _active)))
  (return _output_get))

(fn `UserConstructionScript`)